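; Key-locked sliding door Blueprint that includes its own key pickup, positioned by KeyLocation in the construction script.
; Overlapping KeyBox sets HasKey and destroys the key component.
; Door Box begin and end overlaps share a FlipFlop, alternately playing a Timeline that lerps the door sideways and reversing it after a delay.
; Without the key, those overlaps print a warning message.
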(event `self.Box.OnComponentBeginOverlap`
  (params (OverlappedComponent :type "PrimitiveComponent Object Reference") (OtherActor :type "Actor Object Reference") (OtherComp :type "PrimitiveComponent Object Reference") (OtherBodyIndex :type Integer) (bFromSweep :type Boolean) (SweepResult :type "HitResult Structure (by ref)"))
  ;[0.3121 1 0.3351] DoorSlide
  (if (`self.HasKey?`) :!label _label
    (`/Engine/EditorBlueprintResources/StandardMacros.FlipFlop`
      (:`A`
        (bind (_direction _speed) (`Timeline|Timeline` :!label _label_2)
          (:`Update`
            (`SceneComponent.K2_SetRelativeLocation` (`self.Door`) (`KismetMathLibrary.VLerp` (0.0 0.0 0.0) (200.0 0.0 0.0) _speed) false false))))
      (:`B`
        (`KismetSystemLibrary.Delay` 3.0)
        (goto _label_2 :!via `Reverse`)))
    (else
      (`KismetSystemLibrary.PrintString` "No Key, Please get the key first." true true (struct :`R` 1.0 :`B` 0.053265 :`A` 1.0)))))

(event `self.Box.OnComponentEndOverlap`
  (params (OverlappedComponent :type "PrimitiveComponent Object Reference") (OtherActor :type "Actor Object Reference") (OtherComp :type "PrimitiveComponent Object Reference") (OtherBodyIndex :type Integer))
  ;[0.3121 1 0.3351] DoorSlide
  (goto _label))

(event `self.KeyBox.OnComponentBeginOverlap`
  (params (OverlappedComponent :type "PrimitiveComponent Object Reference") (OtherActor :type "Actor Object Reference") (OtherComp :type "PrimitiveComponent Object Reference") (OtherBodyIndex :type Integer) (bFromSweep :type Boolean) (SweepResult :type "HitResult Structure (by ref)"))
  ;[1 0.1635 0.2332] GetKey
  (set `self.HasKey?` true)
  (`ActorComponent.K2_DestroyComponent` (`self.Key`))
  (`KismetSystemLibrary.PrintString` "Noob you got a Key." true true (struct :`R` 0.082624 :`G` 1.0 :`A` 1.0)))

(event `self.KeyBox.OnComponentEndOverlap`
  (params (OverlappedComponent :type "PrimitiveComponent Object Reference") (OtherActor :type "Actor Object Reference") (OtherComp :type "PrimitiveComponent Object Reference") (OtherBodyIndex :type Integer))
  ;[1 0.1635 0.2332] GetKey
)

(fn `UserConstructionScript`
  (`SceneComponent.K2_SetRelativeLocation` (`self.KeyBox`) (`self.KeyLocation`) false false))